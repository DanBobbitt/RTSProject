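; ControlZoneGrid is a hex tile grid that places a ControlZoneHex actor on every tile.
; The construction script rebuilds a rectangle, hexagon, triangle or parallelogram coordinate array, adding instanced or individual meshes and optional coordinate debug text.
; Each tile's child actor is mapped by coordinate and receives the dynamic material stored for that tile.
; GetControlZoneHexAtCoords actually takes a static mesh, reverse-looking up its coordinate to return the zone.
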(fn `AddControlZoneToHex`
  (params (coords :type "OffsetCoords Structure"))
  (locals (CoordsLocal :type "OffsetCoords Structure"))
  (set `local.CoordsLocal` coords)
  (set `self.CleanTiles` (`self.Grid`))
  (bind _returnvalue (`AddComponent|NODE_AddChildActorComponent-0` :`RelativeTransform` (`KismetMathLibrary.MakeTransform` (`KismetMathLibrary.Conv_Vector2DToVector` (`GridsHex.ScaleAndOffset` (`local.CoordsLocal`) (`KismetMathLibrary.Conv_VectorToVector2D` (`self.GridScaleCalculated`)))) (struct) (`self.PerTileScale`))))
  (`ChildActorComponent.SetChildActorClass` _returnvalue "/Game/Timewar/Blueprints/Core/ControlZoneHex.ControlZoneHex_C")
  (bind _ascontrol_zone_hex (cast `/Game/Timewar/Blueprints/Core/ControlZoneHex` (`ChildActorComponent.ChildActor` _returnvalue) :!pure true))
  (`BlueprintMapLibrary.Map_Add` (`self.ControlZoneMap`) (`local.CoordsLocal`) _ascontrol_zone_hex)
  (set `/Game/Timewar/Blueprints/Core/ControlZoneHex.MaterialInstance` (`BlueprintMapLibrary.Map_Find` (`self.DMIMap`) (`local.CoordsLocal`)) _ascontrol_zone_hex))

(fn `GetControlZoneHexAtCoords`
  (params (`Static Mesh` :type "StaticMeshComponent Object Reference"))
  (returns (`Control Zone` :type "/Game/Timewar/Blueprints/Core/ControlZoneHex Object Reference"))
  (bind _values (`BlueprintMapLibrary.Map_Values` (`self.StaticMeshMap`)))
  (bind _keys (`BlueprintMapLibrary.Map_Keys` (`self.StaticMeshMap`)))
  (return (`BlueprintMapLibrary.Map_Find` (`self.ControlZoneMap`) (`|GetArrayItem` _keys (`KismetArrayLibrary.Array_Find` _values `Static Mesh`)))))

(fn `UserConstructionScript`
  (bind (_gridscale_x _gridscale_y _gridscale_z) (`KismetMathLibrary.BreakVector` (`self.GridScale`)))
  (bind _gridsize (`self.GridSize`))
  (`|ExecutionSequence`
    (:`then_0`
      ;[1 1 1] If using instances, add component and set mesh and material. For a multi-instance setup, see the MultiInstanceExample blueprint
      (if (`self.UseInstances`)
        (bind _returnvalue (`AddComponent|NODE_AddInstancedStaticMeshComponent-0` :`RelativeTransform` (`KismetMathLibrary.MakeTransform` (0.0 0.0 0.0))))
        (bind _output_get (set `self.InstanceComponent` _returnvalue))
        (`StaticMeshComponent.SetStaticMesh` _output_get (`self.BaseTileMesh`))
        (`PrimitiveComponent.SetMaterial` _output_get 0 (`self.BaseTileMaterial`))))
    (:`then_1`
      ;[1 1 1] Clean up previous construction script maps and arrays
      (`BlueprintSetLibrary.Set_Clear` (`self.TileBlockedSet`))
      (`BlueprintMapLibrary.Map_Clear` (`self.TileCostMap`))
      (`KismetArrayLibrary.Array_Clear` (`self.Grid`))
      (`BlueprintMapLibrary.Map_Clear` (`self.StaticMeshMap`))
      (`BlueprintMapLibrary.Map_Clear` (`self.DMIMap`))
      (`BlueprintMapLibrary.Map_Clear` (`self.InstanceMap`)))
    (:`then_2`
      ;[1 1 1] When using perfect hexagons, auto-calculating X from Y gives the perfect spacing.
      (set `self.GridScaleCalculated` (select `bool` (`self.CalculateGridXScale`) :`false` (`self.GridScale`) :`true` (`KismetMathLibrary.MakeVector` (`GridsHex.HexWidth` _gridscale_y) _gridscale_y _gridscale_z))))
    (:`then_3`
      ;[1 1 1] Generate a Grid
      (switch `EHexGridShape` (`self.GridShape`)
        (:`HexGrids_Rectangle`
          (bind _returnvalue_2 (`GridsHex.BuildRectangleArray` _gridsize (`self.CenterGrid`)))
          (set `self.Grid` _returnvalue_2))
        (:`HexGrids_Hexagon`
          (bind _returnvalue_3 (`GridsHex.BuildHexagonArray` _gridsize))
          (set `self.Grid` _returnvalue_3))
        (:`HexGrids_Triangle`
          (bind _returnvalue_4 (`GridsHex.BuildTriangleArray` _gridsize))
          (set `self.Grid` _returnvalue_4))
        (:`HexGrids_Parallelogram`
          (bind _returnvalue_5 (`GridsHex.BuildParallelogramArray` _gridsize (`self.CenterGrid`)))
          (set `self.Grid` _returnvalue_5)))
      ;[1 1 1] Add either an instance or static mesh.
      (for (_array_element _array_index) (`self.Grid`)
        (if (`self.UseInstances`)
          (`self.AddInstance` _array_element)
          (else
            (`self.AddStaticMesh` _array_element)))
        (`self.AddControlZoneToHex` _array_element)
        ;[1 1 1] For Debugging, we can add some text to each tile showing either offset or cube coords
        (switch `/HexGrids/HexGrids/Blueprints/E_DebugText` (`self.DebugType`)
          (:`NewEnumerator1`
            (`self.AddDebugOffsetCoords` _array_element _array_index))
          (:`NewEnumerator2`
            (`self.AddDebugCubeCoords` _array_element)))))))