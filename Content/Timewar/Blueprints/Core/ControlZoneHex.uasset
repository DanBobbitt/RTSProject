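; ControlZoneHex is a hex control zone that tracks the units on it and which team holds it.
; AddUnit moves a unit out of its previous zone into this one, RemoveUnit clears it, and both call UpdateTeam.
; UpdateTeam counts red and blue units to set Team as red, blue or mixed, tinting the material instance to match.
; With neither team counted, Team and color stay unchanged.
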(event `self.ReceiveTick`
  (params (DeltaSeconds :type "Float (single-precision)")))

(event `AddUnit`
  (params (Unit :type "/Game/Timewar/Blueprints/Units/Unit_Base Object Reference"))
  (bind _currentcontrolzone (`/Game/Timewar/Blueprints/Units/Unit_Base.CurrentControlZone` Unit))
  (if (not (`KismetArrayLibrary.Array_Contains` (`self.UnitsPresent`) Unit))
    (`/Engine/EditorBlueprintResources/StandardMacros.IsValid` _currentcontrolzone
      (:`Is Valid`
        (`self.RemoveUnit` _currentcontrolzone Unit))
      (:`Is Not Valid`
        _))
    (`KismetArrayLibrary.Array_Add` (`self.UnitsPresent`) Unit)
    (set `/Game/Timewar/Blueprints/Units/Unit_Base.CurrentControlZone` self Unit)
    (`self.UpdateTeam`)))

(event `RemoveUnit`
  (params (Unit :type "/Game/Timewar/Blueprints/Units/Unit_Base Object Reference"))
  (`KismetArrayLibrary.Array_RemoveItem` (`self.UnitsPresent`) Unit)
  (set `/Game/Timewar/Blueprints/Units/Unit_Base.CurrentControlZone` null Unit)
  (`self.UpdateTeam`))

(fn `UpdateTeam`
  (locals (`Red Team Units` :type Integer) (`Blue Team Units` :type Integer))
  (bind _returnvalue (> (`local.Blue Team Units`) 0))
  (for _array_element (`self.UnitsPresent`)
    (switch `int` (`/Game/Timewar/Blueprints/Units/Unit_Base.Team` _array_element)
      (:`1`
        (`/Engine/EditorBlueprintResources/StandardMacros.IncrementInt` (`local.Red Team Units`)))
      (:`2`
        (`/Engine/EditorBlueprintResources/StandardMacros.IncrementInt` (`local.Blue Team Units`)))))
  (if (> (`local.Red Team Units`) 0)
    (if _returnvalue
      (set `self.Color` (struct :`R` 1.0 :`B` 0.777805 :`A` 1.0))
      (set `self.Team` 3)
      (else
        (set `self.Color` (struct :`R` 1.0 :`A` 1.0))
        (set `self.Team` 1)))
    (`MaterialInstanceDynamic.SetVectorParameterValue` (`self.MaterialInstance`) "Color" (`self.Color`) :!label _label)
    (elif _returnvalue
      (set `self.Color` (struct :`B` 1.0 :`A` 1.0))
      (set `self.Team` 2)
      (goto _label))))

(fn `UserConstructionScript`)