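; Formation designator actor that previews and commits placement of the player's unplaced and selected units.
; On BeginPlay it spawns a phantom waypoint per unit.
; Each tick it faces the cursor, lays waypoints in centred, ground-traced rows that widen with cursor distance, and switches their widgets by spawn-volume overlap.
; PlaceUnits sends existing units to their waypoints and spawns new ones not overlapping cover; CancelPlacement returns unplaced units to the palette.
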(event `self.ReceiveBeginPlay`
  (bind _cursor (`/Game/Timewar/Blueprints/Core/TW_PlayerController_Lobby.Cursor` (`self.ControllingPlayer`)))
  (set `self.UnitInstances` (`/Game/Timewar/Widgets/ScreenElements/Cursor.SelectedUnitsInstances` _cursor))
  (bind _units (`/Game/Timewar/Widgets/ScreenElements/Cursor.RemoveAllUnplacedUnits` _cursor))
  (set `self.UnplacedUnits` _units)
  (for _array_element (`self.UnplacedUnits`)
    (bind (_unitclass _count) (break `/Game/Timewar/Blueprints/Structs/Unit` _array_element))
    (for _ (range 1 (+ _count 1))
      (bind _returnvalue (`|SpawnActorFromClass` "/Game/Timewar/Blueprints/Core/PhantomPlacementWaypoint.PhantomPlacementWaypoint_C" (`self.GetTransform`) "AlwaysSpawn" "OverrideRootScale" null _unitclass null null))
      (`KismetArrayLibrary.Array_Add` (`self.PlacementWaypoints`) _returnvalue)))
  (for _array_element_2 (`self.UnitInstances`)
    (bind _returnvalue_2 (`|SpawnActorFromClass` "/Game/Timewar/Blueprints/Core/PhantomPlacementWaypoint.PhantomPlacementWaypoint_C" (`self.GetTransform`) "AlwaysSpawn" "OverrideRootScale" null (`GameplayStatics.GetObjectClass` _array_element_2) _array_element_2 null))
    (`KismetArrayLibrary.Array_Add` (`self.PlacementWaypoints`) _returnvalue_2)))

(event `self.ReceiveTick`
  (params (DeltaSeconds :type "Float (single-precision)"))
  (`self.Update`))

(fn `CancelPlacement`
  (for _array_element (`self.UnplacedUnits`)
    (bind (_unitclass _count) (break `/Game/Timewar/Blueprints/Structs/Unit` _array_element))
    (for _ (range 1 (+ _count 1))
      (`/Game/Timewar/Widgets/ScreenElements/UnitPalette.AddUnitToPalette` (`/Game/Timewar/Widgets/Screens/LobbyMenu.UnitPalette` (`/Game/Timewar/Blueprints/Core/TW_PlayerController_Lobby.LobbyWidget` (`self.ControllingPlayer`))) (make `/Game/Timewar/Blueprints/Structs/Unit` _unitclass))
      (for _array_element_2 (`self.PlacementWaypoints`)
        (`self.SetLifeSpan` _array_element_2 0.1)))))

(fn `GetClosestEntryPoint`
  (params (Cover :type "/Game/Timewar/Blueprints/Structures+Cover/Cover_Base Object Reference") (Unit :type "/Game/Timewar/Blueprints/Units/Unit_Base Object Reference"))
  (returns (NewParam :type "Vector Structure"))
  (locals (distance :type "Float (double-precision)" :default 100000000.0) (entrypoint :type "/Game/Timewar/Blueprints/Structures+Cover/EntryPoint Object Reference"))
  (for _array_element (`/Game/Timewar/Blueprints/Structures+Cover/Cover_Base.EntryPoints` Cover)
    (bind _returnvalue (`KismetMathLibrary.VSize` (- (`SceneComponent.K2_GetComponentLocation` _array_element) (`self.K2_GetActorLocation` Unit))))
    (if (< _returnvalue (`local.distance`))
      (set `local.distance` _returnvalue)
      (set `local.entrypoint` _array_element)))
  (return (`SceneComponent.K2_GetComponentLocation` (`local.entrypoint`))))

(fn `PlaceUnits`
  (for _array_element (`self.PlacementWaypoints`)
    (bind _owningunitinstance (`/Game/Timewar/Blueprints/Core/PhantomPlacementWaypoint.OwningUnitInstance` _array_element))
    (`/Engine/EditorBlueprintResources/StandardMacros.IsValid` _owningunitinstance
      (:`Is Valid`
        (`/Game/Timewar/Blueprints/Core/TW_PlayerController_Lobby.Send Unit a Waypoint` (`self.ControllingPlayer`) _owningunitinstance (`self.K2_GetActorLocation` _array_element)))
      (:`Is Not Valid`
        (`/Engine/EditorBlueprintResources/StandardMacros.IsValid` (`/Game/Timewar/Blueprints/Core/PhantomPlacementWaypoint.OverlappedCover` _array_element)
          (:`Is Not Valid`
            (`/Game/Timewar/Blueprints/Core/TW_PlayerController_Lobby.Spawn Unit` (`self.ControllingPlayer`) (`/Game/Timewar/Blueprints/Core/PhantomPlacementWaypoint.OwningUnit` _array_element) (`self.GetTransform` _array_element))))))
    (`self.SetLifeSpan` _array_element 0.01)))

(fn `Update`
  (locals (Rows :type "Array of Integer") (RowIndex :type Integer))
  (bind _spread (`self.Spread`))
  (bind _spread_2 (`self.Spread`))
  (bind _returnvalue (`SceneComponent.K2_GetComponentLocation` (`self.DefaultSceneRoot`)))
  (bind _hitresult (`PlayerController.GetHitResultUnderCursorByChannel` (`self.ControllingPlayer`) "TraceTypeQuery1" false))
  (bind _returnvalue_2 (* 2 (`KismetMathLibrary.FTrunc` (/ (`KismetMathLibrary.VSize` (- (`.Location` (`GameplayStatics.BreakHitResult` _hitresult)) _returnvalue)) 1000.0))))
  ;[1 1 1] Set Designator rotation based on player's cursor.
  (if (== 0 _returnvalue_2)
    (`self.K2_SetActorRotation` (`KismetMathLibrary.FindLookAtRotation` _returnvalue _returnvalue))
    (else
      (`self.K2_SetActorRotation` (`KismetMathLibrary.FindLookAtRotation` _returnvalue (`.Location` (`GameplayStatics.BreakHitResult` _hitresult))))))
  ;[1 1 1] Increase number of columns the further the cursor is from the designator.
  (set `self.MaxColumnsInRow` (+ _returnvalue_2 1))
  (for _array_element (`self.PlacementWaypoints`)
    (if (== (`KismetArrayLibrary.Array_Length` (`local.Rows`)) 0)
      (`KismetArrayLibrary.Array_Add` (`local.Rows`))
      (bind _out_hit_location (`self.SetLocationToGround` (.x (`KismetMathLibrary.TransformLocation` (`self.GetTransform`) (`KismetMathLibrary.MakeVector` 0.0))) (.y (`KismetMathLibrary.TransformLocation` (`self.GetTransform`) (`KismetMathLibrary.MakeVector` 0.0))) (.z (`KismetMathLibrary.TransformLocation` (`self.GetTransform`) (`KismetMathLibrary.MakeVector` 0.0))) (`self.PlacementWaypoints`))
        (:`Ground Found`
          (`self.K2_SetActorTransform` _array_element (`KismetMathLibrary.MakeTransform` _out_hit_location) false false)
          (if (`PrimitiveComponent.IsOverlappingActor` (`/Game/Timewar/Blueprints/Core/SpawnVolume.Box` (`/Game/Timewar/Blueprints/Core/TW_PlayerController_Lobby.SpawnVolume` (`self.ControllingPlayer`))) _array_element) :!label _label
            (bind _switcher (`/Game/Timewar/Widgets/ModularObjects/UnitPlacerWidget.Switcher` (cast `/Game/Timewar/Widgets/ModularObjects/UnitPlacerWidget` (`WidgetComponent.GetUserWidgetObject` (`/Game/Timewar/Blueprints/Core/PhantomPlacementWaypoint.Widget` _array_element)) :!pure true)))
            (`WidgetSwitcher.SetActiveWidgetIndex` _switcher 1)
            (else
              (`WidgetSwitcher.SetActiveWidgetIndex` _switcher 2)))))
      (else
        (if (== (`|GetArrayItem` (`local.Rows`) (`local.RowIndex`)) (`self.MaxColumnsInRow`))
          (`KismetArrayLibrary.Array_Add` (`local.Rows`))
          (bind _result (`/Engine/EditorBlueprintResources/StandardMacros.IncrementInt` (`local.RowIndex`))
            (:`  `
              (bind _out_hit_location_2 (`self.SetLocationToGround` (.x (`KismetMathLibrary.TransformLocation` (`self.GetTransform`) (`KismetMathLibrary.MakeVector` (* (* _result -1) (`self.Spread`))))) (.y (`KismetMathLibrary.TransformLocation` (`self.GetTransform`) (`KismetMathLibrary.MakeVector` (* (* _result -1) (`self.Spread`))))) (.z (`KismetMathLibrary.TransformLocation` (`self.GetTransform`) (`KismetMathLibrary.MakeVector` (* (* _result -1) (`self.Spread`))))) (`self.PlacementWaypoints`))
                (:`Ground Found`
                  (`self.K2_SetActorTransform` _array_element (`KismetMathLibrary.MakeTransform` _out_hit_location_2) false false)
                  (goto _label))
                (:`No Ground Found`
                  _))))
          (else
            (bind _result_2 (`/Engine/EditorBlueprintResources/StandardMacros.IncrementInt` (`|GetArrayItem` (`local.Rows`) (`local.RowIndex`)))
              (:`  `
                (if (== (mod _result_2 2) 0)
                  (bind _out_hit_location_3 (`self.SetLocationToGround` (.x (`KismetMathLibrary.TransformLocation` (`self.GetTransform`) (`KismetMathLibrary.MakeVector` (* (* (`local.RowIndex`) -1) _spread_2) (* (/ (`|GetArrayItem` (`local.Rows`) (`local.RowIndex`)) -2) _spread_2)))) (.y (`KismetMathLibrary.TransformLocation` (`self.GetTransform`) (`KismetMathLibrary.MakeVector` (* (* (`local.RowIndex`) -1) _spread_2) (* (/ (`|GetArrayItem` (`local.Rows`) (`local.RowIndex`)) -2) _spread_2)))) (.z (`KismetMathLibrary.TransformLocation` (`self.GetTransform`) (`KismetMathLibrary.MakeVector` (* (* (`local.RowIndex`) -1) _spread_2) (* (/ (`|GetArrayItem` (`local.Rows`) (`local.RowIndex`)) -2) _spread_2)))) (`self.PlacementWaypoints`))
                    (:`Ground Found`
                      (`self.K2_SetActorTransform` _array_element (`KismetMathLibrary.MakeTransform` _out_hit_location_3) false false)
                      (goto _label))
                    (:`No Ground Found`
                      _))
                  (else
                    (bind _out_hit_location_4 (`self.SetLocationToGround` (.x (`KismetMathLibrary.TransformLocation` (`self.GetTransform`) (`KismetMathLibrary.MakeVector` (* (* (`local.RowIndex`) -1) _spread) (* (/ (+ (`|GetArrayItem` (`local.Rows`) (`local.RowIndex`)) 1) 2) _spread)))) (.y (`KismetMathLibrary.TransformLocation` (`self.GetTransform`) (`KismetMathLibrary.MakeVector` (* (* (`local.RowIndex`) -1) _spread) (* (/ (+ (`|GetArrayItem` (`local.Rows`) (`local.RowIndex`)) 1) 2) _spread)))) (.z (`KismetMathLibrary.TransformLocation` (`self.GetTransform`) (`KismetMathLibrary.MakeVector` (* (* (`local.RowIndex`) -1) _spread) (* (/ (+ (`|GetArrayItem` (`local.Rows`) (`local.RowIndex`)) 1) 2) _spread)))) (`self.PlacementWaypoints`))
                      (:`Ground Found`
                        (`self.K2_SetActorTransform` _array_element (`KismetMathLibrary.MakeTransform` _out_hit_location_4) false false)
                        (goto _label))
                      (:`No Ground Found`
                        _))))))))
        (`KismetSystemLibrary.PrintText` "No Ground Found!")))))

(fn `UserConstructionScript`)