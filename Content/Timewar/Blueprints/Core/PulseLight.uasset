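; PulseLight is a light Blueprint that produces a pulse of colored light which shrinks away over time.
; The PulseLight event sets intensity, color and a per-tick falloff, then resets the attenuation radius to its maximum.
; Tick subtracts that falloff from the radius, clamped at zero, so the fade speed depends on frame rate.
; The event's Priority input is unused.
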(event `self.ReceiveTick`
  (params (DeltaSeconds :type "Float (single-precision)"))
  (`self.SetAttenuationRadius` (`KismetMathLibrary.FClamp` (- (`self.AttenuationRadius`) (`self.Falloff Per Tick`)) 0.0 2000.0)))

(event `Pulse Light`
  (params (Intensity :type "Float (double-precision)") (`faloff per tick` :type "Float (double-precision)") (color :type "LinearColor Structure") (priority :type Integer))
  (`self.SetIntensity` Intensity)
  (set `self.Falloff Per Tick` `faloff per tick`)
  (`self.SetLightColor` self color true)
  (`self.SetAttenuationRadius` 2000.0))