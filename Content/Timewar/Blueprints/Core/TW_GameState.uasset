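; Timewar game state that tracks active units, handling their spawning, removal, and server-side visibility.
; On authority, Tick uses a Delay to refresh visibility about every quarter second.
; Each unit adds others as relevant targets when within its vision radius with an unblocked line trace, removing them otherwise.
; A downward trace also finds the hex beneath each unit in the ControlZoneGrid and registers the unit with it.
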(event `self.ReceiveBeginPlay`
  (bind _outactors (`GameplayStatics.GetAllActorsOfClass` "/Game/Timewar/Blueprints/Core/ControlZoneGrid.ControlZoneGrid_C"))
  (set `self.ControlZoneGrid` (`|GetArrayItem` _outactors)))

(event `self.ReceiveTick`
  (params (DeltaSeconds :type "Float (single-precision)"))
  (`/Engine/EditorBlueprintResources/ActorMacros.Switch Has Authority`
    (:`Authority`
      (`KismetSystemLibrary.Delay` 0.25)
      (`self.UpdateUnitVisibility`))))

(event `Spawn Unit`
  (params (`Unit Class` :type "/Game/Timewar/Blueprints/Units/Unit_Base Class Reference") (Transform :type "Transform Structure"))
  (bind _returnvalue (`|SpawnActorFromClass` `Unit Class` Transform "AdjustIfPossibleButAlwaysSpawn" "OverrideRootScale" self null))
  (`KismetArrayLibrary.Array_Add` (`self.ActiveUnits`) _returnvalue))

(event `Unspawn Unit`
  (params (Unit :type "/Game/Timewar/Blueprints/Units/Unit_Base Object Reference"))
  (for _array_element (`self.ActiveUnits`)
    (`/Game/Timewar/Blueprints/Units/Unit_Base.RemoveRelevantTarget` _array_element Unit)
    (`KismetArrayLibrary.Array_RemoveItem` (`self.ActiveUnits`) Unit)
    (`self.SetLifeSpan` Unit 0.1)))

(fn `UpdateUnitVisibility`
  (for _array_element (`self.ActiveUnits`)
    (for _array_element_2 (`self.ActiveUnits`)
      (if (< (`self.GetDistanceTo` _array_element_2 _array_element) (`/Game/Timewar/Blueprints/Units/Unit_Base.VisionRadius` _array_element))
        (bind (_outhit _returnvalue) (`KismetSystemLibrary.LineTraceSingle` :`Start` (`self.K2_GetActorLocation` _array_element) :`End` (`self.K2_GetActorLocation` _array_element_2) :`TraceChannel` "TraceTypeQuery5" :`DrawTime` 0.25))
        (if _returnvalue
          (`/Game/Timewar/Blueprints/Units/Unit_Base.RemoveRelevantTarget` _array_element _array_element_2 :!label _label)
          (else
            (`/Game/Timewar/Blueprints/Units/Unit_Base.AddRelevantTarget` _array_element _array_element_2)))
        (else
          (goto _label))))
    (bind _returnvalue_2 (`self.K2_GetActorLocation` _array_element))
    (bind _outhit_2 (`KismetSystemLibrary.LineTraceSingle` :`Start` (`KismetMathLibrary.MakeVector` (.x _returnvalue_2) (.y _returnvalue_2) (+ (.z _returnvalue_2) 1000.0)) :`End` (`KismetMathLibrary.MakeVector` (.x _returnvalue_2) (.y _returnvalue_2) (- (.z _returnvalue_2) 100000.0)) :`TraceChannel` "TraceTypeQuery7" :`DrawTime` 0.25))
    (bind _asstatic_mesh_component (cast `StaticMeshComponent` (`.HitComponent` (`GameplayStatics.BreakHitResult` _outhit_2))))
    (bind _control_zone (`/Game/Timewar/Blueprints/Core/ControlZoneGrid.GetControlZoneHexAtCoords` (`self.ControlZoneGrid`) _asstatic_mesh_component))
    (`/Game/Timewar/Blueprints/Core/ControlZoneHex.AddUnit` _control_zone _array_element)))

(fn `UserConstructionScript`)