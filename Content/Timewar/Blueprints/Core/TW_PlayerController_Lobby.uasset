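; Lobby player controller for an RTS, covering the lobby, unit setup and in-match unit orders.
; Post-login events build the lobby widget and cursor, claim a free SpawnVolume and possess an RTS camera.
; Army, ready state and chat route through the lobby GameMode, while update events refresh the widget.
; Left mouse selects or box-selects units, right mouse drives a placement grid, and spawned waypoints queue move, attack-move or garrison orders.
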(event `InputAction|OpenInGameMenu`
  (params (Key :type "Key Structure")))

(event `Post Login Client`
  (params (ServerName :type Text))
  ;[1 1 1 1 32] Clientside Updates
  ;;[1 1 1] Setup lobby menu
  (`self.ClientSetHUD` "/Game/Timewar/Widgets/Non-Widgets/MyHud.MyHud_C")
  (set `self.bShowMouseCursor` true)
  (bind _returnvalue (`|CreateWidget` "/Game/Timewar/Widgets/Screens/LobbyMenu.LobbyMenu_C" self ServerName))
  (bind _output_get (set `self.LobbyWidget` _returnvalue))
  (`UserWidget.AddToViewport` _output_get 0)
  (`WidgetBlueprintLibrary.SetInputMode_GameAndUIEx` self (`self.LobbyWidget`))
  (`self.Server Update Player Info`)
  (`/Engine/EditorBlueprintResources/StandardMacros.IsValid` (`self.Cursor`)
    (:`Is Valid`
      _)
    (:`Is Not Valid`
      (bind _returnvalue_2 (`|CreateWidget` "/Game/Timewar/Widgets/ScreenElements/Cursor.Cursor_C" self))
      (bind _output_get_2 (set `self.Cursor` _returnvalue_2))))
  (`self.SetMouseCursorWidget` "Default" _output_get_2))

(event `self.ReceiveEndPlay`
  (params (EndPlayReason :type "EEndPlayReason Enum" :default "Destroyed"))
  ;[1 1 1] Call when disconnected or kicked
  (`DestroySessionCallbackProxy.DestroySession` self :!label _label))

(event `Server Update Player Army`
  (params (`Player Army` :type "/Game/Timewar/Blueprints/Structs/Army Structure"))
  ;[1 1 1] Update Selected Army
  (set `self.SelectedArmy` `Player Army`)
  (`/Game/Timewar/Blueprints/Core/TW_GameMode_Lobby.UpdateAllPlayerInfo` (cast `/Game/Timewar/Blueprints/Core/TW_GameMode_Lobby` (`GameplayStatics.GetGameMode`) :!pure true)))

(event `Server Update Player Info`
  (bind _astw_game_mode_lobby (cast `/Game/Timewar/Blueprints/Core/TW_GameMode_Lobby` (`GameplayStatics.GetGameMode`) :!pure true))
  ;[1 1 1] Update player info on server
  (`/Game/Timewar/Blueprints/Core/TW_GameMode_Lobby.UpdateAllPlayerInfo` _astw_game_mode_lobby)
  (`/Game/Timewar/Blueprints/Core/TW_GameMode_Lobby.TryStartGame` _astw_game_mode_lobby))

(event `Kicked`
  ;[1 1 1] Call when disconnected or kicked
  (`GameplayStatics.OpenLevel` "MainMenu")
  (goto _label))

(event `GetChatMessage`
  (params (TextToSend :type Text))
  (bind _playerinfo_playername (break `/Game/Timewar/Blueprints/Structs/PlayerInfo` (`self.PlayerInfo`)))
  ;[1 1 1] Handle Chat Box
  (set `self.SenderText` TextToSend)
  (set `self.SenderName` _playerinfo_playername)
  (bind _astw_game_mode_lobby (cast `/Game/Timewar/Blueprints/Core/TW_GameMode_Lobby` (`GameplayStatics.GetGameMode`)))
  (for _array_element (`/Game/Timewar/Blueprints/Core/TW_GameMode_Lobby.AllPlayerControllers` _astw_game_mode_lobby)
    (bind _astw_player_controller_lobby (cast `/Game/Timewar/Blueprints/Core/TW_PlayerController_Lobby` _array_element))
    (`self.UpdateChat` _astw_player_controller_lobby (`self.SenderName`) (`self.SenderText`))))

(event `Key|RightMouseButton`
  (params (Key :type "Key Structure"))
  ;[1 1 1] Right Mouse Click (Order Designator)
  (:`Pressed`
    (`self.RightClickPressed`))
  (:`Released`
    (`self.RightClickReleased`)))

(event `UpdatePlayerList`
  (params (ConnectedPlayersInfo :type "Array of /Game/Timewar/Blueprints/Structs/PlayerInfo Structure") (ConnectedPlayerArmies :type "Array of /Game/Timewar/Blueprints/Structs/Army Structure"))
  (bind _lobbywidget (`self.LobbyWidget`))
  ;[1 1 1 1 32] Clientside Updates
  ;;[1 1 1] Update player list
  (set `self.AllConnectedPlayers` ConnectedPlayersInfo)
  (`/Engine/EditorBlueprintResources/StandardMacros.IsValid` _lobbywidget
    (:`Is Valid`
      (`/Game/Timewar/Widgets/Screens/LobbyMenu.ClearPlayerWindow` _lobbywidget)
      (for (_array_element _array_index) (`self.AllConnectedPlayers`)
        (`/Game/Timewar/Widgets/Screens/LobbyMenu.AddPlayerToPlayerWindow` _lobbywidget _array_element (`|GetArrayItem` ConnectedPlayerArmies _array_index))))))

(event `Post Login Server`
  ;[1 1 1] On Post Login
  (bind _outactors (`GameplayStatics.GetAllActorsOfClass` "/Game/Timewar/Blueprints/Core/SpawnVolume.SpawnVolume_C"))
  (for _array_element _outactors
    (bind _asspawn_volume (cast `/Game/Timewar/Blueprints/Core/SpawnVolume` _array_element :!pure true))
    (`/Engine/EditorBlueprintResources/StandardMacros.IsValid` (`/Game/Timewar/Blueprints/Core/SpawnVolume.OccupyingPlayer` _asspawn_volume)
      (:`Is Not Valid`
        (set `/Game/Timewar/Blueprints/Core/SpawnVolume.OccupyingPlayer` self _asspawn_volume)
        (set `self.SpawnVolume` _asspawn_volume)
        (break))))
  (`/Engine/EditorBlueprintResources/StandardMacros.IsValid` (`self.SpawnVolume`)
    (:`Is Valid`
      (bind _returnvalue (`|SpawnActorFromClass` "/Game/Timewar/Blueprints/Core/RTS_Camera.RTS_Camera_C" (`SceneComponent.K2_GetComponentToWorld` (`/Game/Timewar/Blueprints/Core/SpawnVolume.CameraSpawn` (`self.SpawnVolume`))) "AlwaysSpawn" "OverrideRootScale" null null))
      (`self.Possess` self _returnvalue)
      (bind _outactors_2 (`GameplayStatics.GetAllActorsOfClass` "/Game/Timewar/Blueprints/Core/ControlZoneGrid.ControlZoneGrid_C"))
      (set `self.ControlZoneGrid` (`|GetArrayItem` _outactors_2)))
    (:`Is Not Valid`
      (`KismetSystemLibrary.PrintString` "Error! No SpawnVolume found to spawn in a Player" true true (struct :`R` 1.0 :`G` 0.040611 :`A` 1.0)))))

(event `Key|LeftMouseButton`
  (params (Key :type "Key Structure"))
  ;[1 1 1] Left Mouse Click (Selection)
  (:`Pressed`
    (`self.LeftClickPressed`)
    (`KismetSystemLibrary.RetriggerableDelay` 0.1)
    (if (`self.IsInputKeyDown` Key)
      (`self.LeftClickHeld`)))
  (:`Released`
    (`self.LeftClickReleased`)))

(event `UpdateMatchSettings`
  (params (`Map Image` :type "Texture2D Object Reference") (`Map Name` :type Text) (`Map Time` :type Text))
  (bind _lobbywidget (`self.LobbyWidget`))
  ;[1 1 1 1 32] Clientside Updates
  ;;[1 1 1] Update match settings
  (set `/Game/Timewar/Widgets/Screens/LobbyMenu.MapImage` `Map Image` _lobbywidget)
  (set `/Game/Timewar/Widgets/Screens/LobbyMenu.MapName` `Map Name` _lobbywidget)
  (set `/Game/Timewar/Widgets/Screens/LobbyMenu.MapTime` `Map Time` _lobbywidget))

(event `Spawn Unit`
  (params (`Unit class` :type "/Game/Timewar/Blueprints/Units/Unit_Base Class Reference") (transform :type "Transform Structure"))
  ;[1 1 1] Spawn Unit
  (`/Game/Timewar/Blueprints/Core/TW_GameState.Spawn Unit` (cast `/Game/Timewar/Blueprints/Core/TW_GameState` (`GameplayStatics.GetGameState`) :!pure true) `Unit class` transform))

(event `UpdateNumberOfPlayers`
  (params (CurrentPlayers :type Integer) (MaxPlayers :type Integer))
  (bind _lobbywidget (`self.LobbyWidget`))
  ;[1 1 1 1 32] Clientside Updates
  ;;[1 1 1] Update connected players
  (`/Engine/EditorBlueprintResources/StandardMacros.IsValid` _lobbywidget
    (:`Is Valid`
      (set `/Game/Timewar/Widgets/Screens/LobbyMenu.PlayersDisplay` (`|FormatText` "{Current Players} out of {Max Players}" (`KismetTextLibrary.Conv_IntToText` CurrentPlayers) (`KismetTextLibrary.Conv_IntToText` MaxPlayers)) _lobbywidget))))

(event `Key|Four`
  (params (Key :type "Key Structure")))

(event `Send Unit a Waypoint`
  (params (Unit :type "/Game/Timewar/Blueprints/Units/Unit_Base Object Reference") (Location :type "Vector Structure"))
  ;[1 1 1] Send Unit a Waypoint
  (bind _returnvalue (`|SpawnActorFromClass` "/Game/Timewar/Blueprints/Core/OrderWaypoint.OrderWaypoint_C" (`KismetMathLibrary.MakeTransform` Location) "Undefined" "OverrideRootScale" self null))
  (if (`self.IsInputKeyDown` "A")
    (set `/Game/Timewar/Blueprints/Core/OrderWaypoint.Attackmove` true _returnvalue))
  (`/Game/Timewar/Blueprints/Units/Unit_Base.Queue New Order` Unit (not (`self.IsInputKeyDown` "LeftShift")) _returnvalue))

(event `SetPlayerArmy`
  (params (Army :type "/Game/Timewar/Blueprints/Structs/Army Structure"))
  ;[1 1 1 1 32] Clientside Updates
  ;;[1 1 1] Set Player Army
  (set `self.SelectedArmy` Army))

(event `Send Unit a Garrison Waypoint`
  (params (Unit :type "/Game/Timewar/Blueprints/Units/Unit_Base Object Reference") (Location :type "Vector Structure") (`Cover to Garrison` :type "/Game/Timewar/Blueprints/Structures+Cover/Cover_Base Object Reference"))
  ;[1 1 1] Send Unit a Garrison Order
  (bind _returnvalue (`|SpawnActorFromClass` "/Game/Timewar/Blueprints/Core/OrderWaypoint.OrderWaypoint_C" (`KismetMathLibrary.MakeTransform` Location) "Undefined" "OverrideRootScale" null null))
  (if (`self.IsInputKeyDown` "A")
    (set `/Game/Timewar/Blueprints/Core/OrderWaypoint.Attackmove` true _returnvalue))
  (set `/Game/Timewar/Blueprints/Core/OrderWaypoint.ActorOfInterest` `Cover to Garrison` _returnvalue)
  (set `/Game/Timewar/Blueprints/Core/OrderWaypoint.OrderType` "NewEnumerator4" _returnvalue)
  (`/Game/Timewar/Blueprints/Units/Unit_Base.Queue New Order` Unit (not (`self.IsInputKeyDown` "LeftShift")) _returnvalue))

(event `UpdateChat`
  (params (Sender :type Text) (Text :type Text))
  ;[1 1 1 1 32] Clientside Updates
  ;;[1 1 1] Update chat
)

(event `Begin Setup Phase`
  ;[1 1 1] Enter Setup Phase
  (`/Game/Timewar/Widgets/Screens/LobbyMenu.Begin Setup Phase` (`self.LobbyWidget`)))

(event `Begin Game Phase`
  ;[1 1 1] Enter Game Phase
  (`/Game/Timewar/Widgets/Screens/LobbyMenu.Begin Game` (`self.LobbyWidget`)))

(event `ToggleReady`
  (params (Ready :type Boolean))
  ;[1 1 1] Toggle Ready
  (set `self.SetupReady?` Ready)
  (`self.Server Update Player Info`))

(fn `LeftClickHeld`
  (set `/Game/Timewar/Widgets/Non-Widgets/MyHud.DragSelect` true (cast `/Game/Timewar/Widgets/Non-Widgets/MyHud` (`self.GetHUD`) :!pure true)))

(fn `LeftClickPressed`
  (bind _placerdesignator (`self.PlacerDesignator`))
  (bind _cursor (`self.Cursor`))
  (bind (_locationx _locationy) (`self.GetMousePosition` self))
  (`/Game/Timewar/Widgets/ScreenElements/Cursor.RemoveAllSelectedUnits` _cursor)
  (bind _units (`/Game/Timewar/Widgets/ScreenElements/Cursor.RemoveAllUnplacedUnits` _cursor))
  (for _array_element _units
    (bind (_unitclass _count) (break `/Game/Timewar/Blueprints/Structs/Unit` _array_element))
    (for _ (range 1 (+ _count 1))
      (`/Game/Timewar/Widgets/ScreenElements/UnitPalette.AddUnitToPalette` (`/Game/Timewar/Widgets/Screens/LobbyMenu.UnitPalette` (`self.LobbyWidget`)) (make `/Game/Timewar/Blueprints/Structs/Unit` _unitclass))))
  (`/Engine/EditorBlueprintResources/StandardMacros.IsValid` _placerdesignator
    (:`Is Valid`
      (`/Game/Timewar/Blueprints/Core/UnitPlacerGrid.CancelPlacement` _placerdesignator)
      (`self.K2_DestroyActor` _placerdesignator)
      (set `self.PlacerDesignator` null))
    (:`Is Not Valid`
      (bind _asunit_base (cast `/Game/Timewar/Blueprints/Units/Unit_Base` (`.HitActor` (`GameplayStatics.BreakHitResult` (`self.GetHitResultUnderCursorByChannel` "TraceTypeQuery2" false))))
        (:`then`
          (`self.SelectUnit` _asunit_base))
        (:`CastFailed`
          _))
      (set `/Game/Timewar/Widgets/Non-Widgets/MyHud.dragstart` (`KismetMathLibrary.MakeVector2D` _locationx _locationy) (cast `/Game/Timewar/Widgets/Non-Widgets/MyHud` (`self.GetHUD`) :!pure true)))))

(fn `LeftClickReleased`
  (bind (_locationx _locationy) (`self.GetMousePosition`))
  (bind _asmy_hud (cast `/Game/Timewar/Widgets/Non-Widgets/MyHud` (`self.GetHUD`) :!pure true))
  (set `/Game/Timewar/Widgets/Non-Widgets/MyHud.dragend` (`KismetMathLibrary.MakeVector2D` _locationx _locationy) _asmy_hud)
  (set `/Game/Timewar/Widgets/Non-Widgets/MyHud.DragSelect` false _asmy_hud)
  (return))

(fn `RemoveUnitFromSelection`
  (params (Unit :type "/Game/Timewar/Blueprints/Units/Unit_Base Object Reference"))
  (locals (PhantomWaypoint :type "/Game/Timewar/Blueprints/Core/PhantomPlacementWaypoint Object Reference"))
  (if (`KismetArrayLibrary.Array_Contains` (`/Game/Timewar/Widgets/ScreenElements/Cursor.SelectedUnitsInstances` (`self.Cursor`)) Unit)
    (`/Game/Timewar/Widgets/ScreenElements/Cursor.RemoveSelectedUnitFromCursor` (`self.Cursor`) Unit)
    (`/Engine/EditorBlueprintResources/StandardMacros.IsValid` (`self.PlacerDesignator`))))

(fn `RightClickPressed`
  (bind (_hitresult _returnvalue) (`self.GetHitResultUnderCursorByChannel` "TraceTypeQuery6"))
  (if (and _returnvalue (not (`|EnumEquality` (`/Game/Timewar/Blueprints/Core/TW_GameState.GameStatus` (cast `/Game/Timewar/Blueprints/Core/TW_GameState` (`GameplayStatics.GetGameState`) :!pure true)) "NewEnumerator0")))
    (`self.Spawn Unit Placer` (`.Location` (`GameplayStatics.BreakHitResult` _hitresult)))))

(fn `RightClickReleased`
  (bind _placerdesignator (`self.PlacerDesignator`))
  (`/Engine/EditorBlueprintResources/StandardMacros.IsValid` _placerdesignator
    (:`Is Valid`
      (`/Game/Timewar/Blueprints/Core/UnitPlacerGrid.PlaceUnits` _placerdesignator)
      (`self.K2_DestroyActor` _placerdesignator)
      (set `self.PlacerDesignator` null))))

(fn `SelectUnit`
  (params (UnitBase :type "/Game/Timewar/Blueprints/Units/Unit_Base Object Reference"))
  (`/Game/Timewar/Widgets/ScreenElements/Cursor.AddSelectedUnitToCursor` (`self.Cursor`) UnitBase))

(fn `SelectUnitsInABox`
  (params (Start :type "Vector2D Structure") (End :type "Vector2D Structure"))
  (for _array_element (`HUD.GetActorsInSelectionRectangle` (`self.GetHUD`) "/Game/Timewar/Blueprints/Units/Unit_Base.Unit_Base_C" Start End false false)
    (bind _asunit_base (cast `/Game/Timewar/Blueprints/Units/Unit_Base` _array_element))
    (`/Game/Timewar/Widgets/ScreenElements/Cursor.AddSelectedUnitToCursor` (`self.Cursor`) _asunit_base)))

(fn `UserConstructionScript`)