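; Base actor for a squad member (module) of a parent unit, which follows it in formation, takes cover and fights.
; Tick moves it toward a randomized, ground-snapped formation offset, or through a cover state machine between entry point and assigned firing port.
; It turns toward targets picked randomly from enemy modules, with the server toggling its in-range weapons.
; Hits roll armor penetration against health, and death spawns a corpse.
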(event `self.ReceiveTick`
  (params (DeltaSeconds :type "Float (single-precision)"))
  (if (`/Game/Timewar/Blueprints/Units/Unit_Base.InCover?` (`self.ParentUnit`))
    (`self.UpdatePositionInCover` DeltaSeconds
      (:`Out`
        _))
    (else
      (`self.UpdatePosition` DeltaSeconds)))
  (`self.AimAndEngageTarget` DeltaSeconds))

(event `self.Collision.OnComponentBeginOverlap`
  (params (OverlappedComponent :type "PrimitiveComponent Object Reference") (OtherActor :type "Actor Object Reference") (OtherComp :type "PrimitiveComponent Object Reference") (OtherBodyIndex :type Integer) (bFromSweep :type Boolean) (SweepResult :type "HitResult Structure (by ref)"))
  (bind _reservedcover (`/Game/Timewar/Blueprints/Units/Unit_Base.ReservedCover` (`self.ParentUnit`)))
  (`/Engine/EditorBlueprintResources/StandardMacros.IsValid` _reservedcover
    (:`Is Valid`
      (if (and (== _reservedcover OtherActor) (`ActorComponent.ComponentHasTag` OtherComp "EntryPoint"))
        (switch `/Game/Timewar/Blueprints/Enums/ModuleStatesInCover` (`self.CoverStatus`)
          (:`NewEnumerator0`
            (bind _firingposition (`/Game/Timewar/Blueprints/Structures+Cover/Cover_Base.AssignModuleToFiringPort` (`/Game/Timewar/Blueprints/Units/Unit_Base.ReservedCover` (`self.ParentUnit`)) self))
            (set `self.CoverFiringPoint` _firingposition)
            (set `self.CoverStatus` "NewEnumerator1"))
          (:`NewEnumerator2`
            (set `self.CoverStatus` "NewEnumerator3")
            (set `self.CoverFiringPoint` null)
            (`KismetSystemLibrary.PrintString` "NOT IN COVER SET")))))))

(event `Update Desired Offset`
  (params (`Random X` :type "Float (double-precision)") (`Random Y` :type "Float (double-precision)") (Radius :type "Float (double-precision)"))
  (set `self.(Relative) Desired Offset` (+ (`self.(Relative) Formation Slot`) (* (`KismetMathLibrary.MakeVector` `Random X` `Random Y`) Radius))))

(event `self.ReceiveBeginPlay`
  (`/Engine/EditorBlueprintResources/ActorMacros.Switch Has Authority`
    (:`Authority`
      (`self.Update Desired Offset` (`KismetMathLibrary.RandomFloatInRange` -1.0 1.0) (`KismetMathLibrary.RandomFloatInRange` -1.0 1.0) 100.0)
      (`SceneComponent.K2_SetWorldLocation` (`self.DefaultSceneRoot`) (+ (`self.K2_GetActorLocation` (`self.ParentUnit`)) (`self.(Relative) Desired Offset`)) false false))))

(event `/Game/Timewar/Blueprints/Core/Damageable.Recieve Attack`
  (params (`Damage Amount` :type Integer) (Penetration :type Integer) (`Damage Type` :type Text))
  (bind _returnvalue (- (`self.Health`) `Damage Amount`))
  (if (> (`self.Health`) 0)
    (`self.Penetrated?` Penetration
      (:`Success`
        (if (<= _returnvalue 0)
          (`self.Module Death`))
        (set `self.Health` _returnvalue))
      (:`Failed`
        (`KismetSystemLibrary.PrintString` "Ricochet!")))))

(event `Module Death`
  (bind _returnvalue (`|SpawnActorFromClass` "/Game/Timewar/Blueprints/Modules/Corpse_Base.Corpse_Base_C" (`SceneComponent.K2_GetComponentToWorld` (`self.DefaultSceneRoot`)) "AdjustIfPossibleButAlwaysSpawn" "OverrideRootScale" null null))
  (`/Game/Timewar/Blueprints/Modules/Corpse_Base.Initialization` _returnvalue)
  (`KismetArrayLibrary.Array_RemoveItem` (`/Game/Timewar/Blueprints/Units/Unit_Base.ModuleActors` (`self.ParentUnit`)) self)
  (for _array_element _
    (`self.K2_DestroyActor` _array_element))
  (`ActorComponent.K2_DestroyComponent` (`self.GetParentComponent`))
  (`self.K2_DestroyActor`))

(event `Target Random Module`
  (params (`Target Unit` :type "/Game/Timewar/Blueprints/Units/Unit_Base Object Reference"))
  (bind _moduleactors (`/Game/Timewar/Blueprints/Units/Unit_Base.ModuleActors` `Target Unit`))
  (bind _returnvalue (`KismetArrayLibrary.Array_Length` _moduleactors))
  (bind _output (`|GetArrayItem` _moduleactors (`KismetMathLibrary.RandomIntegerInRange` 0 (- _returnvalue 1))))
  (`/Engine/EditorBlueprintResources/StandardMacros.DoOnce` false :!label _label
    (:`Completed`
      (if (> _returnvalue 0)
        (if (> (`/Game/Timewar/Blueprints/Modules/Module_Base.Health` _output) 0)
          (set `self.CurrentTarget` _output)
          (`KismetSystemLibrary.Delay` 2.0)
          (goto _label :!via `Reset`)
          (else
            (goto _label :!via `Reset`)))
        (else
          (set `self.CurrentTarget` null)
          (goto _label :!via `Reset`))))))

(fn `AddModule`
  (params (EquipmentBase :type "/Game/Timewar/Blueprints/Equipment/Equipment_Base Object Reference"))
  (`KismetArrayLibrary.Array_Add` (`self.EquipmentActors`) EquipmentBase)
  (bind _asweapon_base (cast `/Game/Timewar/Blueprints/Equipment/Weapon_Base` EquipmentBase))
  (bind _maxrange (`/Game/Timewar/Blueprints/Equipment/Weapon_Base.MaxRange` _asweapon_base))
  (if (> _maxrange (`self.LargestRange`))
    (set `self.LargestRange` _maxrange)))

(fn `UserConstructionScript`)