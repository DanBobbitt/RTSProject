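; Base class for a Timewar unit: a moving group of child-actor modules that fights and follows queued waypoint orders.
; Construction spawns the modules; on BeginPlay the server attaches type-checked equipment to their sockets.
; During one game status, server tick has modules target within the closest relevant enemy unit or other unit, and the unit dies when no modules remain.
; Waypoint orders drive AI movement, advancing on capsule overlap.
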(event `self.ReceiveBeginPlay`
  ;[1 1 1] Initial Setup
  (`WidgetSwitcher.SetActiveWidgetIndex` (`/Game/Timewar/Widgets/ModularObjects/UnitWidget.WidgetSwitcher_0` (cast `/Game/Timewar/Widgets/ModularObjects/UnitWidget` (`WidgetComponent.GetUserWidgetObject` (`self.Unit Icon`)) :!pure true)) 6)
  (`/Engine/EditorBlueprintResources/ActorMacros.Switch Has Authority`
    (:`Authority`
      (for _array_element (`self.EquipmentSlots`)
        (`self.VerifyEquipmentSlot` (break `/Game/Timewar/Blueprints/Core/EquipmentSlot` _array_element) (`.EquipmentType_10_9E6C386349CADA91BA0C1FAC763D06F8` (break `/Game/Timewar/Blueprints/Core/EquipmentSlot` _array_element))
          (:`Verified`
            (`self.AttachEquipmentToModule` (break `/Game/Timewar/Blueprints/Core/EquipmentSlot` _array_element) (`.ModuleName_5_F856C18C42073CC817F363A6134BB7B0` (break `/Game/Timewar/Blueprints/Core/EquipmentSlot` _array_element)) (`.SocketName_11_C48F682748D9B4AF79F90B8A0E839801` (break `/Game/Timewar/Blueprints/Core/EquipmentSlot` _array_element)))))))))

(event `self.ReceiveTick`
  (params (DeltaSeconds :type "Float (single-precision)"))
  (bind _returnvalue (`self.GetVelocity`))
  (`/Engine/EditorBlueprintResources/ActorMacros.Switch Has Authority`
    (:`Authority`
      (if (== (`KismetArrayLibrary.Array_Length` (`self.ModuleActors`)) 0)
        (`/Engine/EditorBlueprintResources/StandardMacros.DoOnce` false
          (:`Completed`
            (`self.Unit Death`)))
        (else
          (`self.Target Management On Tick`)
          (if (> (`KismetMathLibrary.VSize` _returnvalue) 10.0)
            (`SceneComponent.K2_SetWorldRotation` (`self.UnitToken`) (`KismetMathLibrary.MakeRotFromX` _returnvalue) false false)))))))

(event `Queue New Order`
  (params (`Clear Previous Orders` :type Boolean) (`Order Waypoint` :type "/Game/Timewar/Blueprints/Core/OrderWaypoint Object Reference"))
  (`self.Queue Order` `Clear Previous Orders` `Order Waypoint`))

(event `self.CapsuleComponent.OnComponentBeginOverlap`
  (params (OverlappedComponent :type "PrimitiveComponent Object Reference") (OtherActor :type "Actor Object Reference") (OtherComp :type "PrimitiveComponent Object Reference") (OtherBodyIndex :type Integer) (bFromSweep :type Boolean) (SweepResult :type "HitResult Structure (by ref)"))
  (`/Engine/EditorBlueprintResources/ActorMacros.Switch Has Authority`
    (:`Authority`
      (bind _asorder_waypoint (cast `/Game/Timewar/Blueprints/Core/OrderWaypoint` OtherActor))
      (`self.PassOverWaypoint` _asorder_waypoint))))

(fn `AddRelevantTarget`
  (params (`Target Actor` :type "Actor Object Reference (by ref)"))
  (bind _asunit_base (cast `/Game/Timewar/Blueprints/Units/Unit_Base` `Target Actor`))
  (if (not (== _asunit_base self))
    (`KismetArrayLibrary.Array_Add` (`self.RelevantTargets`) _asunit_base)))

(fn `ExecuteOrder`
  (if (> (`KismetArrayLibrary.Array_Length` (`self.Waypoints`)) 0)
    (`NavigationSystem.SimpleMoveToActor` (`AIBlueprintHelperLibrary.GetAIController` self) (`|GetArrayItem` (`self.Waypoints`)))))

(fn `PassOverWaypoint`
  (params (`Order Waypoint` :type "/Game/Timewar/Blueprints/Core/OrderWaypoint Object Reference"))
  (bind _output (`|GetArrayItem` (`self.Waypoints`)))
  (if (== `Order Waypoint` _output)
    (if (> (`KismetArrayLibrary.Array_Length` (`self.Waypoints`)) 1)
      (`self.K2_DestroyActor` (`|GetArrayItem` (`self.Waypoints`)))
      (`KismetArrayLibrary.Array_Remove` (`self.Waypoints`))
      (`self.ExecuteOrder`)
      (else
        (`SceneComponent.K2_SetWorldRotation` (`self.Mesh`) (`self.K2_GetActorRotation` _output) false false)
        (`self.K2_DestroyActor` (`|GetArrayItem` (`self.Waypoints`)))
        (`KismetArrayLibrary.Array_Remove` (`self.Waypoints`))
        (`MovementComponent.StopMovementImmediately` (`self.CharacterMovement`))))))

(fn `Queue Order`
  (params (`Clear Previous Order` :type Boolean) (`Order Waypoint` :type "/Game/Timewar/Blueprints/Core/OrderWaypoint Object Reference"))
  (if `Clear Previous Order`
    (for _array_element (`self.Waypoints`)
      (`self.SetLifeSpan` _array_element 0.1))
    (`KismetArrayLibrary.Array_Clear` (`self.Waypoints`))
    (`KismetArrayLibrary.Array_Add` (`self.Waypoints`) `Order Waypoint`)
    (if (`|EnumEquality` (`/Game/Timewar/Blueprints/Core/TW_GameState.GameStatus` (cast `/Game/Timewar/Blueprints/Core/TW_GameState` (`GameplayStatics.GetGameState`) :!pure true)) "NewEnumerator3") :!label _label
      (`self.ExecuteOrder`))
    (else
      (bind _returnvalue (`KismetArrayLibrary.Array_Add` (`self.Waypoints`) `Order Waypoint`))
      (if (== _returnvalue 0)
        (goto _label)))))

(fn `RemoveRelevantTarget`
  (params (`Target Actor` :type "Actor Object Reference (by ref)"))
  (bind _asunit_base (cast `/Game/Timewar/Blueprints/Units/Unit_Base` `Target Actor`))
  (`KismetArrayLibrary.Array_RemoveItem` (`self.RelevantTargets`) _asunit_base)
  ;[1 1 1] Unset current target for relevant child modules
  (for _array_element (`self.ModuleActors`)
    (if (== (`/Game/Timewar/Blueprints/Modules+Equipment/Module_Base.CurrentTarget` _array_element) _asunit_base)
      (set `/Game/Timewar/Blueprints/Modules+Equipment/Module_Base.CurrentTarget` null _array_element))))

(fn `Target Management On Tick`
  (locals (ClosestTargetRange :type "Float (double-precision)" :default 1000000000.0))
  (if (`|EnumEquality` (`/Game/Timewar/Blueprints/Core/TW_GameState.GameStatus` (cast `/Game/Timewar/Blueprints/Core/TW_GameState` (`GameplayStatics.GetGameState`) :!pure true)) "NewEnumerator3")
    (set `local.ClosestTargetRange` 100000000.0)
    (for _array_element (`self.RelevantTargets`)
      (bind _returnvalue (`self.GetDistanceTo` self _array_element))
      (if (< _returnvalue (`local.ClosestTargetRange`))
        (set `local.ClosestTargetRange` _returnvalue)
        (set `self.CurrentTarget` _array_element)))
    (`/Engine/EditorBlueprintResources/StandardMacros.IsValid` (`self.CurrentTarget`)
      (:`Is Valid`
        (for _array_element_2 (`self.ModuleActors`)
          (`/Game/Timewar/Blueprints/Modules+Equipment/Module_Base.Target Random Module` _array_element_2 (`self.CurrentTarget`)))))))

(fn `UserConstructionScript`
  ;[1 1 1] Spawn in our modules
  (for _array_element (`self.Modules`)
    (bind _returnvalue (`AddComponent|NODE_AddChildActorComponent-0` :`RelativeTransform` (`.RelativeTransform_24_AF4497CD4D69D5388CEBB4AC154AA4B3` (break `/Game/Timewar/Blueprints/Core/Module` _array_element))))
    (`ChildActorComponent.SetChildActorClass` _returnvalue (`.ModuleClass_19_55BFEBAD4949D2524CCEC99A0C215D30` (break `/Game/Timewar/Blueprints/Core/Module` _array_element)))
    (bind _asmodule_base (cast `/Game/Timewar/Blueprints/Modules+Equipment/Module_Base` (`ChildActorComponent.ChildActor` _returnvalue)))
    (set `/Game/Timewar/Blueprints/Modules+Equipment/Module_Base.(Relative) Formation Slot` (.location (`.RelativeTransform_24_AF4497CD4D69D5388CEBB4AC154AA4B3` (break `/Game/Timewar/Blueprints/Core/Module` _array_element))) _asmodule_base)
    (set `/Game/Timewar/Blueprints/Modules+Equipment/Module_Base.ParentUnit` self _asmodule_base)
    (`KismetArrayLibrary.Array_Add` (`self.ModuleActors`) _asmodule_base)
    (set `/Game/Timewar/Blueprints/Modules+Equipment/Module_Base.ModuleName` (break `/Game/Timewar/Blueprints/Core/Module` _array_element) _asmodule_base)))