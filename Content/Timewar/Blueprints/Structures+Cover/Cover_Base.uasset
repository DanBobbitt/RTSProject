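; Base cover structure Blueprint that lets units occupy firing positions, tracking which unit module holds each one.
; Construction script registers every Arrow component as a key in the FiringPositions map and gathers Sphere components as EntryPoints.
; UnitRequestEntry checks that enough positions are free for all of a unit's modules; AssignModuleToFiringPort claims the first free one and returns its arrow.
; Debug prints report counts and checks.
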(event `self.ReceiveBeginPlay`
  (`KismetSystemLibrary.PrintString` (`KismetStringLibrary.Concat_StrStr` (`KismetStringLibrary.Conv_IntToString` (`BlueprintMapLibrary.Map_Length` (`self.Firing Positions`))) " FP, " (`KismetStringLibrary.Conv_IntToString` (`KismetArrayLibrary.Array_Length` (`self.EntryPoints`))) " EP.") true true (struct :`R` 1.0 :`G` 0.011862 :`A` 1.0) 10.0))

(fn `AssignModuleToFiringPort`
  (params (Module :type "/Game/Timewar/Blueprints/Modules/Module_Base Object Reference"))
  (returns (FiringPosition :type "ArrowComponent Object Reference"))
  (locals (index :type Integer :default -1) (Keys :type "Array of ArrowComponent Object Reference") (Values :type "Array of /Game/Timewar/Blueprints/Modules/Module_Base Object Reference"))
  (bind _values (`BlueprintMapLibrary.Map_Values` (`self.Firing Positions`)))
  (set `local.Values` _values)
  (bind _keys (`BlueprintMapLibrary.Map_Keys` (`self.Firing Positions`)))
  (bind _output_get (set `local.Keys` _keys))
  (for (_array_element _array_index) _output_get
    (bind (_value _returnvalue) (`BlueprintMapLibrary.Map_Find` (`self.Firing Positions`) _array_element))
    (if _returnvalue
      (`/Engine/EditorBlueprintResources/StandardMacros.IsValid` _value
        (:`Is Valid`
          (`KismetSystemLibrary.PrintString` "IsValid"))
        (:`Is Not Valid`
          (`BlueprintMapLibrary.Map_Add` (`self.Firing Positions`) _array_element Module)
          (set `local.index` _array_index)
          (return _array_element)))
      (else
        (`KismetSystemLibrary.PrintString` "Somehow failed to find Firing Position with provided Arrow Component key!")))))

(fn `UnitRequestEntry`
  (params (Unit :type "/Game/Timewar/Blueprints/Units/Unit_Base Object Reference"))
  (returns (EntryGranted :type Boolean))
  (locals (Values :type "Array of /Game/Timewar/Blueprints/Modules/Module_Base Object Reference") (Keys :type "Array of ArrowComponent Object Reference") (ValidValues :type Integer))
  (bind _firing_positions (`self.Firing Positions`))
  (bind _returnvalue (`KismetArrayLibrary.Array_Length` (`/Game/Timewar/Blueprints/Units/Unit_Base.ModuleActors` Unit)))
  (bind _returnvalue_2 (- (`KismetArrayLibrary.Array_Length` (`local.Keys`)) (`local.ValidValues`)))
  (bind _keys (`BlueprintMapLibrary.Map_Keys` _firing_positions))
  (set `local.Keys` _keys)
  (bind _values (`BlueprintMapLibrary.Map_Values` _firing_positions))
  (bind _output_get (set `local.Values` _values))
  (for _array_element _output_get
    (`/Engine/EditorBlueprintResources/StandardMacros.IsValid` _array_element
      (:`Is Valid`
        (`/Engine/EditorBlueprintResources/StandardMacros.IncrementInt` (`local.ValidValues`)))))
  (`KismetSystemLibrary.PrintString` (`KismetStringLibrary.Concat_StrStr` "Entry Check: " (`KismetStringLibrary.Conv_IntToString` _returnvalue_2) ">= " (`KismetStringLibrary.Conv_IntToString` _returnvalue) " ?    Firing Positions count:" (`KismetStringLibrary.Conv_IntToString` (`BlueprintMapLibrary.Map_Length` (`self.Firing Positions`)))))
  (return (>= _returnvalue_2 _returnvalue)))

(fn `UserConstructionScript`
  (for _array_element (`self.K2_GetComponentsByClass` "/Script/Engine.ArrowComponent")
    (`BlueprintMapLibrary.Map_Add` (`self.Firing Positions`) _array_element))
  (set `self.EntryPoints` (`self.K2_GetComponentsByClass` "/Script/Engine.SphereComponent")))